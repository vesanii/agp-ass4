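; Weapon pickup Blueprint that changes the look of its pickup mesh to match the weapon's rarity.
; UpdateWeaponPickupMaterial passes WeaponRarity to a multicast event, which runs the implementation function.
; That function creates a dynamic material instance on slot 0 from the Common, Rare, Master or Legendary material.
; The vector parameter set on each instance has no name, and BeginPlay and the construction script are empty.
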(event `Multicast UpdateWeaponPickupMaterial`
  (params (Rarity :type "EWeaponRarity Enum" :default "Common"))
  (`self.UpdateWeaponPickupMaterialImplementation` Rarity))

(event `self.UpdateWeaponPickupMaterial`
  (`self.Multicast UpdateWeaponPickupMaterial` (`self.WeaponRarity`)))

(event `self.ReceiveBeginPlay`)

(fn `UpdateWeaponPickupMaterialImplementation`
  (params (Rarity :type "EWeaponRarity Enum" :default "Common"))
  (bind _pickupmesh (`self.PickupMesh`))
  (switch `EWeaponRarity` Rarity
    (:`Common`
      (bind _returnvalue (`PrimitiveComponent.CreateDynamicMaterialInstance` _pickupmesh 0 "/Game/Materials/Pickups/CommonMaterial.CommonMaterial" "None"))
      (`MaterialInstanceDynamic.SetVectorParameterValue` :`self` _returnvalue))
    (:`Rare`
      (bind _returnvalue_2 (`PrimitiveComponent.CreateDynamicMaterialInstance` _pickupmesh 0 "/Game/Materials/Pickups/RareMaterial.RareMaterial" "None"))
      (`MaterialInstanceDynamic.SetVectorParameterValue` :`self` _returnvalue_2))
    (:`Master`
      (bind _returnvalue_3 (`PrimitiveComponent.CreateDynamicMaterialInstance` _pickupmesh 0 "/Game/Materials/Pickups/MasterMaterial.MasterMaterial" "None"))
      (`MaterialInstanceDynamic.SetVectorParameterValue` :`self` _returnvalue_3))
    (:`Legendary`
      (bind _returnvalue_4 (`PrimitiveComponent.CreateDynamicMaterialInstance` _pickupmesh 0 "/Game/Materials/Pickups/LegendaryMaterial.LegendaryMaterial" "None"))
      (`MaterialInstanceDynamic.SetVectorParameterValue` :`self` _returnvalue_4))))

(fn `UserConstructionScript`)